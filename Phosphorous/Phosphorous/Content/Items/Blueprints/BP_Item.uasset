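; BP_Item is a world item actor that can be picked up into an inventory and can show its own HUD widget.
; Interact wraps ItemProperties in an inventory slot for the interacter's Inventory_Component, plays the pickup sound regardless of the result, and destroys the actor only if the add succeeds.
; Separate events create and remove the HUD widget from a class reference.
; UseItem and DiscardItem are stubs that return true.
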(event EventBeginPlay)

(event Collision|EventActorBeginOverlap
  (params (OtherActor :type Actor%20Object%20Reference)))

(event EventTick
  (params (DeltaSeconds :type Float%20%28single-precision%29)))

(event EventInteract
  (params (Interacter :type Actor%20Object%20Reference))
  (bind _success (Default|AddtoInventory (Actor|GetComponentbyClass Interacter "/Game/InventorySystem/Inventory_Component.Inventory_Component_C") (Utilities|Struct|MakeST_Slot (Variables|Default|GetitemProperties) (.quantity (Variables|Default|GetitemProperties)))))
  (Audio|PlaySound2D "/Game/MyAssets/Sounds/Menu/Item_PickedUp.Item_PickedUp" 1.0 1.0 0.0 0 0)
  (if _success
    (Actor|DestroyActor)))

(event EventRemoveItemHUDfromScreen
  (Widget|RemovefromParent (Variables|Default|GetItemHUDWidget)))

(event EventEquiptoHUD
  (bind _returnvalue (UserInterface|CreateWidget (Variables|Default|GetItemHUDClassRef)))
  (bind _output_get (Variables|Default|SetItemHUDWidget _returnvalue))
  (UserInterface|Viewport|AddtoViewport _output_get 0))

(fn ConstructionScript)

(fn UseItem
  (return true))

(fn DiscardItem
  (return true))