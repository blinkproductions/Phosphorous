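; BP_BaseNote is a base interactable note actor that shows and hides a note widget on screen.
; Interact calls ToggleNote, which either creates the NoteWidget class centered by anchor and alignment at WidgetPosition, or removes the stored widget and clears its reference.
; Ending overlap with its Box component also closes the note if it is open.
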(event OnComponentEndOverlap(Box)
  (params (OverlappedComponent :type Primitive%20Component%20Object%20Reference) (OtherActor :type Actor%20Object%20Reference) (OtherComp :type Primitive%20Component%20Object%20Reference) (OtherBodyIndex :type Integer))
  (Variables|Default|GetWidgetRef
    (:then
      (CallFunction|ToggleNote))
    (:else)))

(event EventBeginPlay)

(event Collision|EventActorBeginOverlap
  (params (OtherActor :type Actor%20Object%20Reference)))

(event EventTick
  (params (DeltaSeconds :type Float%20%28single-precision%29)))

(event EventInteract
  (params (Interacter :type Actor%20Object%20Reference))
  (CallFunction|ToggleNote))

(fn ConstructionScript)

(fn ToggleNote
  (Variables|Default|GetWidgetRef
    (:then
      (Widget|RemovefromParent (Variables|Default|GetWidgetRef))
      (Variables|Default|SetWidgetRef 0))
    (:else
      (bind _returnvalue (UserInterface|CreateWidget (Variables|Default|GetNoteWidget)))
      (bind _output_get (Variables|Default|SetWidgetRef _returnvalue))
      (UserInterface|Viewport|AddtoViewport _output_get 0)
      (Class|UserWidget|SetAlignmentinViewport (Variables|Default|GetWidgetRef) "(X=0.500000,Y=0.500000)")
      (Class|UserWidget|SetAnchorsinViewport (Variables|Default|GetWidgetRef) (Utilities|Struct|MakeAnchors "(X=0.500000,Y=0.500000)" "(X=0.500000,Y=0.500000)"))
      (Class|UserWidget|SetPositioninViewport (Variables|Default|GetWidgetRef) (Variables|Default|GetWidgetPosition) true))))