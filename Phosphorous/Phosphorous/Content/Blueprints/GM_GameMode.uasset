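; Game mode that respawns the player character and picks the level entry point.
; BeginPlay stores the player's transform in GI_GameInstance, loads persistent inventory and binds to the character's destruction.
; On destruction it waits RespawnDelay, spawns and possesses a new character at that saved transform, then repeats the inventory load and binding.
; ChoosePlayerStart matches PlayerStart tags against the game instance's DoorID, falling back to the first start found.
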(event Custom|Character_Respawn
  (params (DestroyedActor :type Actor%20Object%20Reference))
  (Utilities|FlowControl|Delay (Variables|Default|GetRespawnDelay))
  (bind _returnvalue (Game|SpawnActorfromClass "/Game/Blueprints/BP_MainCharacter_Test.BP_MainCharacter_Test_C" (CallFunction|GetTransformfromInstance) "Undefined" 0 0))
  (Pawn|Possess (Game|GetPlayerController 0) _returnvalue)
  (CallFunction|Respawn))

(event Custom|Respawn
  (bind _asbp_main_character_test (Utilities|Casting|CastToBP_MainCharacter_Test (Game|GetPlayerCharacter 0)))
  (Default|LoadPersistInventory (Variables|/Game/Blueprints/BP_MainCharacter_Test.BP_MainCharacter_Test_C|GetInventory_Component _asbp_main_character_test))
  (Game|BindEventtoOnDestroyed _asbp_main_character_test (delegate Custom|Character_Respawn)))

(event EventBeginPlay
  (bind _asgi_game_instance (Utilities|Casting|CastToGI_GameInstance (Game|GetGameInstance)))
  (Variables|/Game/Blueprints/GI_GameInstance.GI_GameInstance_C|SetRespawnTransformInInstance _asgi_game_instance (Transformation|GetActorTransform (Game|GetPlayerCharacter 0)))
  (bind _asbp_main_character_test (Utilities|Casting|CastToBP_MainCharacter_Test (Game|GetPlayerCharacter 0)))
  (Default|LoadPersistInventory (Variables|/Game/Blueprints/BP_MainCharacter_Test.BP_MainCharacter_Test_C|GetInventory_Component _asbp_main_character_test))
  (Game|BindEventtoOnDestroyed _asbp_main_character_test (delegate Custom|Character_Respawn)))

(event EventTick
  (params (DeltaSeconds :type Float%20%28single-precision%29)))

(fn ConstructionScript)

(fn ChoosePlayerStart
  (params (Player :type Controller%20Object%20Reference))
  (bind _asgi_game_instance (Utilities|Casting|CastToGI_GameInstance (Game|GetGameInstance)))
  (bind _outactors (Actor|GetAllActorsOfClass "/Script/Engine.PlayerStart"))
  (for _array_element _outactors
    (if (Utilities|Name|Equal(Name) (Variables|/Script/Engine.PlayerStart|GetPlayerStartTag _array_element) (Variables|/Game/Blueprints/GI_GameInstance.GI_GameInstance_C|GetDoor_ID _asgi_game_instance))
      (return _array_element)))
  (return (Utilities|Array|Get(acopy) _outactors)))

(fn GetTransformfromInstance
  (bind _asgi_game_instance (Utilities|Casting|CastToGI_GameInstance (Game|GetGameInstance)))
  (return (Variables|/Game/Blueprints/GI_GameInstance.GI_GameInstance_C|GetRespawnTransformInInstance _asgi_game_instance)))