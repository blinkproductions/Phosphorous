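; BP_PlayerSpawn is a level-transition trigger that sends the player to another map through a numbered or named door.
; When BP_MainCharacter_Test overlaps its box collision, it saves that character's persistent inventory and writes its DoorID to GI_GameInstance.
; It then opens the level whose name comes from converting the Destination enum to a string.
; Despite the name, the file contains no spawning logic.
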(event OnComponentBeginOverlap(BoxCollision)
  (params (OverlappedComponent :type Primitive%20Component%20Object%20Reference) (OtherActor :type Actor%20Object%20Reference) (OtherComp :type Primitive%20Component%20Object%20Reference) (OtherBodyIndex :type Integer) (bFromSweep :type Boolean) (SweepResult :type Hit%20Result%20Structure%20%28by%20ref%29))
  (bind _asbp_main_character_test (Utilities|Casting|CastToBP_MainCharacter_Test OtherActor))
  (Default|SavePersistInventory (Variables|/Game/Blueprints/BP_MainCharacter_Test.BP_MainCharacter_Test_C|GetInventory_Component _asbp_main_character_test))
  (bind _asgi_game_instance (Utilities|Casting|CastToGI_GameInstance (Game|GetGameInstance)))
  (Variables|/Game/Blueprints/GI_GameInstance.GI_GameInstance_C|SetDoor_ID _asgi_game_instance (Variables|Default|GetDoor_ID))
  (Game|OpenLevel(byName) (Utilities|String|StringToName (Utilities|String|EnumtoString (Variables|Default|GetDestination)))))

(event EventBeginPlay)

(event Collision|EventActorBeginOverlap
  (params (OtherActor :type Actor%20Object%20Reference)))

(event EventTick
  (params (DeltaSeconds :type Float%20%28single-precision%29)))

(fn ConstructionScript)