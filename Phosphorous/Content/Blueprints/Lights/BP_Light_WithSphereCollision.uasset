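; BP_Light_WithSphereCollision is a powerable spotlight that tells the game mode when the player is inside its light.
; Begin and end overlaps on its Sphere with BP_MainCharacter_Test set PlayerIsInsideLight on GM_GameMode, but only while PowerOn is true.
; Tick shows or hides the spotlight and visualization mesh from PowerOn.
; Logic to toggle sphere collision and VisionRadius is present but disconnected, so the sphere ignores power changes.
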(event OnComponentBeginOverlap(Sphere)
  (params (OverlappedComponent :type Primitive%20Component%20Object%20Reference) (OtherActor :type Actor%20Object%20Reference) (OtherComp :type Primitive%20Component%20Object%20Reference) (OtherBodyIndex :type Integer) (bFromSweep :type Boolean) (SweepResult :type Hit%20Result%20Structure%20%28by%20ref%29))
  (Utilities|Casting|CastToBP_MainCharacter_Test OtherActor)
  (if (Variables|Default|GetbPowerOn)
    (Variables|/Game/Blueprints/GM_GameMode.GM_GameMode_C|SetbPlayerIsInsideLight (Variables|Default|GetGameModeRef) true)))

(event OnComponentEndOverlap(Sphere)
  (params (OverlappedComponent :type Primitive%20Component%20Object%20Reference) (OtherActor :type Actor%20Object%20Reference) (OtherComp :type Primitive%20Component%20Object%20Reference) (OtherBodyIndex :type Integer))
  (Utilities|Casting|CastToBP_MainCharacter_Test OtherActor)
  (if (Variables|Default|GetbPowerOn)
    (Variables|/Game/Blueprints/GM_GameMode.GM_GameMode_C|SetbPlayerIsInsideLight (Variables|Default|GetGameModeRef) false)))

(event EventBeginPlay
  (|CallParentFunction)
  (bind _asgm_game_mode (Utilities|Casting|CastToGM_GameMode (Game|GetGameMode)))
  (Variables|Default|SetGameModeRef _asgm_game_mode))

(event EventTick
  (params (DeltaSeconds :type Float%20%28single-precision%29))
  (bind _spotlight (Variables|Default|GetSpotLight))
  (|CallParentFunction DeltaSeconds)
  (if (Variables|Default|GetbPowerOn)
    (Development|SetHiddeninGame _spotlight false false)
    (else
      (Development|SetHiddeninGame _spotlight true false))))

(fn ConstructionScript)