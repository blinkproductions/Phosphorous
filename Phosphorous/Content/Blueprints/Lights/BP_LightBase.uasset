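; Base light actor that, while powered, checks whether it has line of sight to the player.
; Power is read every tick from the GameInstance's circuit switch array by SwitchIndex.
; LightCheck runs a debug-drawn visibility trace to the player and prints results, but the player-hit branch only casts, with no effect yet.
; BPCLoSVisualizer runs at construction, and getters expose vision radius, angle, orientation vectors and visualization mesh.
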(event EventBeginPlay
  (bind _asgi_game_instance (Utilities|Casting|CastToGI_GameInstance (Game|GetGameInstance)))
  (Variables|Default|SetbPowerOn (Utilities|Array|Get(acopy) (Variables|/Game/Blueprints/GI_GameInstance.GI_GameInstance_C|GetCircuitSwitchIndex _asgi_game_instance) (Variables|Default|GetSwitchIndex)))
  (if (Variables|Default|GetbPowerOn)
    _))

(event EventTick
  (params (DeltaSeconds :type Float%20%28single-precision%29))
  (bind _asgi_game_instance (Utilities|Casting|CastToGI_GameInstance (Game|GetGameInstance)))
  (Variables|Default|SetbPowerOn (Utilities|Array|Get(acopy) (Variables|/Game/Blueprints/GI_GameInstance.GI_GameInstance_C|GetCircuitSwitchIndex _asgi_game_instance) (Variables|Default|GetSwitchIndex)))
  (if (Variables|Default|GetbPowerOn)
    (CallFunction|LightCheck)))

(fn ConstructionScript
  (Default|RunConstructionScript (Variables|Default|GetBPC_LoSVisualizer)))

(fn LightCheck
  (bind _returnvalue (Game|GetPlayerCharacter 0))
  (bind _returnvalue_2 (Transformation|GetActorLocation _returnvalue))
  (bind (_x _y _z) (Math|Vector|BreakVector _returnvalue_2))
  (bind (_outhit _returnvalue_3) (Collision|LineTraceByChannel (Transformation|GetWorldLocation (Variables|Default|GetLightParentPosition)) (Math|Vector|MakeVector _x _y _z) "TraceTypeQuery1" false 0 "ForOneFrame"))
  (if _returnvalue_3
    (Development|PrintString (Utilities|String|Append "(BP_LightBase) Actor hit by trace: " (Utilities|GetDisplayName (.HitActor (Collision|BreakHitResult _outhit)))) true true "(R=0.000000,G=0.660000,B=1.000000,A=1.000000)" 0.0)
    (if (== (.HitActor (Collision|BreakHitResult _outhit)) (.AsTest%20Character%20Backup (Utilities|Casting|CastToTestCharacter_Backup (Game|GetPlayerCharacter 0))))
      (Utilities|Casting|CastToTestCharacter_Backup (Game|GetPlayerCharacter 0))
      (else
        (Development|PrintString "Timer Not Reset!" true true "(R=0.000000,G=0.660000,B=1.000000,A=1.000000)" 0.0)))))

(fn RetrieveVisionParameters
  (return (Variables|Default|GetVisionRadius) (Variables|Default|GetVisionAngle) (Transformation|GetActorForwardVector) (Math|Vector|GetUpVector "0, 0, 0")))

(fn RetrieveVisualizationMeshComponent
  (return (Variables|Default|GetVisualizationMesh)))