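; BP_Light_Point is a point light actor that shows or hides its PointLight component according to a PowerOn flag.
; BeginPlay runs the parent logic, then hides the light if power is off.
; Tick calls the parent, then reapplies visibility every frame by polling PowerOn rather than reacting to changes.
; It also prints the SwitchIndex and power state on screen each frame as debug output.
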(event EventBeginPlay
  (|CallParentFunction)
  (if (not (Variables|Default|GetbPowerOn))
    (Development|SetHiddeninGame (Variables|Default|GetPointLight) true false)))

(event Collision|EventActorBeginOverlap
  (params (OtherActor :type Actor%20Object%20Reference)))

(event EventTick
  (params (DeltaSeconds :type Float%20%28single-precision%29))
  (bind _bpoweron (Variables|Default|GetbPowerOn))
  (bind _pointlight (Variables|Default|GetPointLight))
  (|CallParentFunction DeltaSeconds)
  (Development|PrintString (Utilities|String|Append "(BP_Light_Point) Power on index  " (Utilities|String|ToString(Integer) (Variables|Default|GetSwitchIndex)) ": " (Utilities|String|ToString(Boolean) _bpoweron)) true true "(R=0.000000,G=0.660000,B=1.000000,A=1.000000)" 0.0)
  (if _bpoweron
    (Development|SetHiddeninGame _pointlight false false)
    (else
      (Development|SetHiddeninGame _pointlight true false))))

(fn ConstructionScript
  (|CallParentFunction))