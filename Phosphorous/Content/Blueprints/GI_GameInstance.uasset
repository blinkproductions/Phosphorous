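; Game instance that owns the save system, persisting the player's transform and inventory across sessions.
; On Init it loads the existing save slot into a cached save object, or creates a new one if none exists.
; Save and load functions copy the capsule transform and inventory between the player character and that object, with only saving writing to disk.
; A clear function deletes the slot.
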(event EventInit
  (CallFunction|InitializeSave))

(fn SavePlayerData
  (bind _savegamedata (Variables|Default|GetSaveGameData))
  (bind _asbp_main_character_test (Utilities|Casting|CastToBP_MainCharacter_Test (Game|GetPlayerCharacter 0)))
  (LocalVariables|SetPlayerRef _asbp_main_character_test)
  (Variables|/Game/Blueprints/Saving/SaveGameObject.SaveGameObject_C|SetPlayerData _savegamedata (Utilities|Struct|MakePlayerData (Transformation|GetWorldTransform (Variables|/Script/Engine.Character|GetCapsuleComponent (LocalVariables|GetPlayerRef))) (Variables|Default|GetInventoryData)))
  (SaveGame|SaveGametoSlot _savegamedata (Variables|Default|GetSaveSlotName)))

(fn LoadPlayerData
  (bind _savegamedata (Variables|Default|GetSaveGameData))
  (bind _playerdata (Variables|/Game/Blueprints/Saving/SaveGameObject.SaveGameObject_C|GetPlayerData _savegamedata))
  (bind _asbp_main_character_test (Utilities|Casting|CastToBP_MainCharacter_Test (Game|GetPlayerCharacter 0)))
  (bind _output_get (LocalVariables|SetPlayerRef _asbp_main_character_test))
  (Transformation|SetActorTransform _output_get (.playertransform _playerdata))
  (Variables|Default|SetInventoryData (.playerinventory _playerdata)))

(fn ClearSaveData
  (SaveGame|DeleteGameinSlot (Variables|Default|GetSaveSlotName)))

(fn InitializeSave
  (bind _returnvalue (SaveGame|DoesSaveGameExist (Variables|Default|GetSaveSlotName)))
  (if _returnvalue
    (bind _returnvalue_2 (SaveGame|LoadGamefromSlot (Variables|Default|GetSaveSlotName)))
    (bind _assave_game_object (Utilities|Casting|CastToSaveGameObject _returnvalue_2))
    (Variables|Default|SetSaveGameData _assave_game_object)
    (else
      (bind _returnvalue_3 (SaveGame|CreateSaveGameObject "/Game/Blueprints/Saving/SaveGameObject.SaveGameObject_C"))
      (Variables|Default|SetSaveGameData _returnvalue_3))))