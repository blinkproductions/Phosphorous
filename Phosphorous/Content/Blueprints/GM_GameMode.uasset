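; Game mode that carries player state across level transitions through GI_GameInstance, handling spawn location and inventory restore.
; ChoosePlayerStart picks the PlayerStart whose tag matches the game instance's DoorID, falling back to the first one found.
; BeginPlay has BP_MainCharacter_Test's InventoryComponent load its persisted inventory.
; Tick prints the game instance's inventory on screen as debug output, and a disconnected load path for TestCharacter_Backup remains.
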(event EventBeginPlay
  (Development|PrintString "Hello")
  (bind _asbp_main_character_test (Utilities|Casting|CastToBP_MainCharacter_Test (Game|GetPlayerCharacter 0)))
  (Default|LoadPersistInventory (Variables|/Game/Blueprints/BP_MainCharacter_Test.BP_MainCharacter_Test_C|GetInventory_Component _asbp_main_character_test)))

(event EventTick
  (params (DeltaSeconds :type Float%20%28single-precision%29))
  (Development|PrintString "(GM_GameMode)GAME INSTANCE:" true true "(R=1.000000,G=0.118020,B=0.000000,A=1.000000)" 0.0)
  (bind _asgi_game_instance (Utilities|Casting|CastToGI_GameInstance (Game|GetGameInstance)))
  (for _array_element (Variables|/Game/Blueprints/GI_GameInstance.GI_GameInstance_C|GetInventoryData _asgi_game_instance)
    (Development|PrintString (Utilities|String|Append (Utilities|String|ToString(Name) (.name (.ItemStructure (Utilities|Struct|BreakST_Slot _array_element)))) " " (Utilities|String|ToString(Integer) (.Quantity (Utilities|Struct|BreakST_Slot _array_element)))) true true "(R=1.000000,G=0.116445,B=0.000000,A=1.000000)" 0.0)))

(fn ConstructionScript)

(fn ChoosePlayerStart
  (params (Player :type Controller%20Object%20Reference))
  (bind _asgi_game_instance (Utilities|Casting|CastToGI_GameInstance (Game|GetGameInstance)))
  (bind _outactors (Actor|GetAllActorsOfClass "/Script/Engine.PlayerStart"))
  (for _array_element _outactors
    (if (Utilities|Name|Equal(Name) (Variables|/Script/Engine.PlayerStart|GetPlayerStartTag _array_element) (Variables|/Game/Blueprints/GI_GameInstance.GI_GameInstance_C|GetDoor_ID _asgi_game_instance))
      (return _array_element)))
  (return (Utilities|Array|Get(acopy) _outactors)))