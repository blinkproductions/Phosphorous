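; BP_Item_Camera is a camera item that shows a camera HUD when the player interacts with it.
; BeginPlay caches the game mode and player character, and Interact adds the player's CameraHUDRef to the viewport.
; DiscardItem removes the item's own CameraHUDRef, whose creation code is disconnected and never runs.
; UseItem only returns true.
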(event EventBeginPlay
  (|CallParentFunction)
  (bind _asgm_game_mode (Utilities|Casting|CastToGM_GameMode (Game|GetGameMode)))
  (Variables|Default|SetGameModeRef _asgm_game_mode)
  (bind _asbp_main_character_test (Utilities|Casting|CastToBP_MainCharacter_Test (Game|GetPlayerCharacter 0)))
  (Variables|Default|SetPlayerRef _asbp_main_character_test))

(event Collision|EventActorBeginOverlap
  (params (OtherActor :type Actor%20Object%20Reference))
  (|CallParentFunction OtherActor) ; This node is disabled and will not be called.\nDrag off pins to build functionality.
)

(event EventTick
  (params (DeltaSeconds :type Float%20%28single-precision%29))
  (|CallParentFunction DeltaSeconds))

(event EventInteract
  (params (Interacter :type Actor%20Object%20Reference))
  (|CallParentFunction Interacter)
  (UserInterface|Viewport|AddtoViewport (Variables|/Game/Blueprints/BP_MainCharacter_Test.BP_MainCharacter_Test_C|GetCameraHUDRef (Variables|Default|GetPlayerRef)) 0))

(fn ConstructionScript
  (|CallParentFunction))

(fn UseItem
  (return true))

(fn DiscardItem
  (bind _bsuccess (|CallParentFunction))
  (Widget|RemovefromParent (Variables|Default|GetCameraHUDRef))
  (return _bsuccess))