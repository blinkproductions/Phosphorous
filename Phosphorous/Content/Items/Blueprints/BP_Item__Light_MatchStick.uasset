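; Matchstick light item that gives the player a short-lived, flickering light.
; UseItem plays a strike sound, spawns another instance of this Blueprint to run FlickerLight, and sets MatchLit on the character.
; FlickerLight makes the sphere block a custom trace channel, flags the player as inside light in the game mode and drives intensity by timeline.
; Tick follows the character's MatchAnchor; after LightDuration, flag and collision revert and the actor destroys itself.
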(event Custom|FlickerLight
  ;[1 1 1] makes light flicker
  (Collision|SetCollisionResponsetoChannel (Variables|Default|GetSphere) "ECC_GameTraceChannel1" "ECR_Block")
  (Variables|/Game/Blueprints/GM_GameMode.GM_GameMode_C|SetbPlayerIsInsideLight (Variables|Default|GetGameModeRef) true)
  (Utilities|FlowControl|Delay (Math|Random|RandomFloatinRange 0.0 0.2))
  (bind _intensity (Timeline|Timeline_0 Play)
    (:Update
      (Rendering|Components|Light|SetIntensity (Variables|Default|GetPointLight) (* _intensity 5e+03))
      (Utilities|FlowControl|Delay (Variables|Default|GetLightDuration))
      (Variables|/Game/Blueprints/GM_GameMode.GM_GameMode_C|SetbPlayerIsInsideLight (Variables|Default|GetGameModeRef) false)
      (Collision|SetCollisionResponsetoChannel (Variables|Default|GetSphere) "ECC_GameTraceChannel1" "ECR_Ignore")
      (Actor|DestroyActor))))

(event Custom|FollowAnchorPoint
  (Transformation|SetRelativeLocation (Variables|Default|GetDefaultSceneRoot) (Transformation|GetWorldLocation (Variables|/Game/Blueprints/BP_MainCharacter_Test.BP_MainCharacter_Test_C|GetmatchAnchor (.AsBP%20Main%20Character%20Test (Utilities|Casting|CastToBP_MainCharacter_Test (Game|GetPlayerCharacter 0))))) false false))

(event EventBeginPlay
  (|CallParentFunction)
  (bind _asgm_game_mode (Utilities|Casting|CastToGM_GameMode (Game|GetGameMode)))
  (Variables|Default|SetGameModeRef _asgm_game_mode))

(event Collision|EventActorBeginOverlap
  (params (OtherActor :type Actor%20Object%20Reference))
  (|CallParentFunction OtherActor) ; This node is disabled and will not be called.\nDrag off pins to build functionality.
)

(event EventTick
  (params (DeltaSeconds :type Float%20%28single-precision%29))
  (|CallParentFunction DeltaSeconds)
  (CallFunction|FollowAnchorPoint))

(fn ConstructionScript
  (|CallParentFunction))

(fn UseItem
  (bind _bsuccess (|CallParentFunction))
  (Audio|PlaySound2D "/Game/MyAssets/Sounds/Match_Light.Match_Light" 1.0 1.0 0.0 0 0)
  (bind _returnvalue (Game|SpawnActorfromClass "BP_Item__Light_MatchStick_C" (Math|Transform|MakeTransform "0, 0, 0" "0, 0, 0" "1,1,1") "Undefined" 0 0))
  (CallFunction|FlickerLight _returnvalue)
  (bind _asbp_main_character_test (Utilities|Casting|CastToBP_MainCharacter_Test (Game|GetPlayerCharacter 0)))
  (Variables|/Game/Blueprints/BP_MainCharacter_Test.BP_MainCharacter_Test_C|SetbMatchLit _asbp_main_character_test true)
  (return _bsuccess))